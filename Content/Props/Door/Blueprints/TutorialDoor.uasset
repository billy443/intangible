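; TutorialDoor is a door prop that slides its Door component between a closed start position and an open end position.
; OpenDoor_Event acts as a toggle, playing or reversing a timeline based on the Open flag.
; The timeline lerps the door's relative location and flips Open only when it finishes.
; The construction script places the door at the end position when Open is set.
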(event Custom|OpenDoor_Event
  (if (Variables|Default|GetOpen)
    (bind _driver (Timeline|Timeline%20-%20Door%20Driver Reverse)
      (:Update
        (Transformation|SetRelativeLocation (Variables|Default|GetDoor) (Math|Vector|Lerp(Vector) (Variables|Default|GetDoorStart) (Variables|Default|GetDoorEnd) _driver) false))
      (:Finished
        (if (Variables|Default|GetOpen)
          (Variables|Default|SetOpen false)
          (else
            (Variables|Default|SetOpen true)))))
    (else
      (Timeline|Timeline%20-%20Door%20Driver Play))))

(fn ConstructionScript
  (if (Variables|Default|GetOpen)
    (Transformation|SetRelativeLocation (Variables|Default|GetDoor) (Variables|Default|GetDoorEnd) false)))