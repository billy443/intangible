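; Timed sliding door that moves away from its initial open or closed position when OpenDoor_Event fires, then returns after a delay.
; The construction script places the door at DoorEnd when Open is set, and that flag also picks each timeline's direction.
; TimelineDoorDriver lerps the door between DoorStart and DoorEnd, with DoorDelay triggered from its Update rather than Finished.
; A second timeline, Timeline_0, drives the return movement.
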(event Custom|OpenDoor_Event
  (if (Variables|Default|GetOpen)
    (bind _driver (Timeline|Timeline%20-%20Door%20Driver Reverse)
      (:Update
        (Transformation|SetRelativeLocation (Variables|Default|GetDoor) (Math|Vector|Lerp(Vector) (Variables|Default|GetDoorStart) (Variables|Default|GetDoorEnd) _driver) false)
        (Utilities|FlowControl|Delay (Variables|Default|GetDoorDelay))
        (if (Variables|Default|GetOpen)
          (bind _driver_2 (Timeline|Timeline_0 Play)
            (:Update
              (Transformation|SetRelativeLocation (Variables|Default|GetDoor) (Math|Vector|Lerp(Vector) (Variables|Default|GetDoorStart) (Variables|Default|GetDoorEnd) _driver_2) false)))
          (else
            (Timeline|Timeline_0 Reverse)))))
    (else
      (Timeline|Timeline%20-%20Door%20Driver Play))))

(fn ConstructionScript
  (if (Variables|Default|GetOpen)
    (Transformation|SetRelativeLocation (Variables|Default|GetDoor) (Variables|Default|GetDoorEnd) false)))