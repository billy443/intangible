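; Collectible pickup that, on the first overlap by Main_Character, hides its mesh and raises the player's collectible count, capped at five.
; It writes the count into the character's popup text and shows it briefly using delays.
; At five it boosts the phase meter's maximum and recharge rate and shows a second popup; otherwise it destroys itself afterwards.
; Save-game create and load nodes exist but are unconnected.
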(event EventActorBeginOverlap
  (params (OtherActor :type Actor%20Object%20Reference))
  (if (== (Utilities|GetClass OtherActor) "/Game/Blueprints/Main_Character.Main_Character_C")
    (Utilities|FlowControl|DoOnce false
      (:Completed
        (bind _asmain_character_c (Utilities|Casting|CastToMain_Character OtherActor))
        (Variables|/Game/Blueprints/Main_Character.Main_Character_C|SetPopupText _asmain_character_c (Utilities|String|Append (Utilities|String|Append (Variables|Default|GetFirstString) (Utilities|String|ToString(Integer) (Math|Integer|Clamp(Integer) (+ (Variables|/Game/Blueprints/Main_Character.Main_Character_C|GetCollectibleCount _asmain_character_c) 1) 0 5))) (Variables|Default|GetSecondString)))
        (Variables|/Game/Blueprints/Main_Character.Main_Character_C|SetCollectibleCount _asmain_character_c (Math|Integer|Clamp(Integer) (+ (Variables|/Game/Blueprints/Main_Character.Main_Character_C|GetCollectibleCount _asmain_character_c) 1) 0 5))
        (Rendering|SetVisibility (Variables|Default|GetStaticMesh1) false false)
        (if (>= (Variables|/Game/Blueprints/Main_Character.Main_Character_C|GetCollectibleCount _asmain_character_c) 5)
          (Variables|/Game/Blueprints/Main_Character.Main_Character_C|Setphase_meter_max _asmain_character_c (+ (Variables|/Game/Blueprints/Main_Character.Main_Character_C|Getphase_meter_max _asmain_character_c) 2.0))
          (Variables|/Game/Blueprints/Main_Character.Main_Character_C|Setphase_meter_recharge_rate _asmain_character_c (* (Variables|/Game/Blueprints/Main_Character.Main_Character_C|Getphase_meter_recharge_rate _asmain_character_c) 3.0)))
        (Variables|/Game/Blueprints/Main_Character.Main_Character_C|SetShowPopupText _asmain_character_c true)
        (Utilities|FlowControl|Delay 3.0)
        (Variables|/Game/Blueprints/Main_Character.Main_Character_C|SetShowPopupText _asmain_character_c false)
        (if (>= (Variables|/Game/Blueprints/Main_Character.Main_Character_C|GetCollectibleCount _asmain_character_c) 5)
          (Variables|/Game/Blueprints/Main_Character.Main_Character_C|SetPopupText _asmain_character_c (Variables|Default|GetPhaseString))
          (Utilities|FlowControl|Delay 0.2)
          (Variables|/Game/Blueprints/Main_Character.Main_Character_C|SetShowPopupText _asmain_character_c true)
          (Utilities|FlowControl|Delay 3.0)
          (Variables|/Game/Blueprints/Main_Character.Main_Character_C|SetShowPopupText _asmain_character_c false)
          (else
            (Actor|DestroyActor)))))))

(fn ConstructionScript)