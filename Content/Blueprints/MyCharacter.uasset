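; Side-view player character with a hold-to-phase ability that slows the world while keeping its own speed via compensating time dilation.
; Phasing swaps movement, jump gravity, visible mesh and capsule collision type.
; Overlap events count collisions, save the entry location and detect traps; releasing phase inside objects snaps back, or damages inside traps.
; Zero HP triggers death animation and level load; debug keys alter camera grading and activation.
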(event Input|ActionEvents|InputActionphase
  (bind _returnvalue (Game|GetPlayerCharacter 0))
  (bind _skeletalmesh1 (Variables|Character|GetSkeletalMesh1))
  (bind _charactermovement (Variables|Character|GetCharacterMovement))
  (bind _mesh (Variables|Character|GetMesh))
  (bind _capsulecomponent (Variables|/Script/Engine.Character|GetCapsuleComponent _returnvalue))
  (:Pressed
    (Variables|Default|Setphase true)
    ;[1 1 1] Enable/Disable Time Dilation
    (Utilities|Time|SetGlobalTimeDilation 0.33)
    (Variables|Default|SetCustomTimeDilation 3.0)
    ;[1 1 1] Enable/Disable Phase Movement Changes
    (Variables|/Script/Engine.CharacterMovementComponent|SetMaxWalkSpeed _charactermovement (Variables|Default|Getphase_walk_speed))
    (Variables|/Script/Engine.CharacterMovementComponent|SetMaxAcceleration _charactermovement (Variables|Default|Getphase_acceleration))
    (Variables|/Script/Engine.CharacterMovementComponent|SetJumpZVelocity _charactermovement (Variables|Default|Getphase_jump_velocity))
    (Rendering|SetCastShadow _mesh false)
    (Rendering|SetVisibility _mesh false false)
    (Rendering|SetVisibility _skeletalmesh1 true false)
    (Collision|SetCollisionObjectType _capsulecomponent "ECC_Vehicle"))
  (:Released
    (Variables|Default|Setphase false)
    (Utilities|Time|SetGlobalTimeDilation 1.0)
    (Variables|Default|SetCustomTimeDilation 1.0)
    (Variables|/Script/Engine.CharacterMovementComponent|SetMaxWalkSpeed _charactermovement (Variables|Default|Getnormal_walk_speed))
    (Variables|/Script/Engine.CharacterMovementComponent|SetMaxAcceleration _charactermovement (Variables|Default|Getnormal_acceleration))
    (Variables|/Script/Engine.CharacterMovementComponent|SetJumpZVelocity _charactermovement (Variables|Default|Getnormal_jump_velocity))
    (Rendering|SetCastShadow _mesh true)
    (Rendering|SetVisibility _mesh true false)
    (Rendering|SetVisibility _skeletalmesh1 false false)
    (Collision|SetCollisionObjectType _capsulecomponent "ECC_Pawn")
    (if (and (not (Variables|Default|GetinTrap)) (> (Variables|Default|Getcollision_count) 0.0))
      (Transformation|SetActorLocation (Variables|Default|Getphase_start_location) false)
      (elif (Variables|Default|GetinTrap)
        (Utilities|TakeDamage)))))

(event EventOnLanded
  (params (Hit :type Hit%20Result%20Structure%20%28by%20ref%29))
  (if (not (Variables|Default|Getphase))
    (Variables|/Script/Engine.CharacterMovementComponent|SetGravityScale (Variables|Character|GetCharacterMovement) (Variables|Default|Getnormal_gravity))))

(event EventOnJumped
  (bind _charactermovement (Variables|Character|GetCharacterMovement))
  (if (Variables|Default|Getphase)
    (Variables|/Script/Engine.CharacterMovementComponent|SetGravityScale _charactermovement (Variables|Default|Getphase_gravity))
    (else
      (Variables|/Script/Engine.CharacterMovementComponent|SetGravityScale _charactermovement (Variables|Default|Getnormal_gravity)))))

(event Input|KeyboardEvents|LeftCtrl)

(event Input|KeyboardEvents|LeftAlt
  (bind _sideviewcameracomponent (Variables|Default|GetSideViewCameraComponent))
  (bind _postprocesssettings (Variables|/Script/Engine.CameraComponent|GetPostProcessSettings _sideviewcameracomponent))
  (bind (_boverride_filmwhitepoint _boverride_filmsaturation _boverride_filmchannelmixerred _boverride_filmchannelmixergreen _boverride_filmchannelmixerblue _boverride_filmcontrast _boverride_filmdynamicrange _boverride_filmhealamount _boverride_filmtoeamount _boverride_filmshadowtint _boverride_filmshadowtintblend _boverride_filmshadowtintamount _boverride_scenecolortint _boverride_scenefringeintensity _boverride_scenefringesaturation _boverride_ambientcubemaptint _boverride_ambientcubemapintensity _boverride_bloomintensity _boverride_bloomthreshold _boverride_bloom1tint _boverride_bloom1size _boverride_bloom2size _boverride_bloom2tint _boverride_bloom3tint _boverride_bloom3size _boverride_bloom4tint _boverride_bloom4size _boverride_bloom5tint _boverride_bloom5size _boverride_bloomdirtmaskintensity _boverride_bloomdirtmasktint _boverride_bloomdirtmask _boverride_autoexposurelowpercent _boverride_autoexposurehighpercent _boverride_autoexposureminbrightness _boverride_autoexposuremaxbrightness _boverride_autoexposurespeedup _boverride_autoexposurespeeddown _boverride_autoexposurebias _boverride_histogramlogmin _boverride_histogramlogmax _boverride_lensflareintensity _boverride_lensflaretint _boverride_lensflaretints _boverride_lensflarebokehsize _boverride_lensflarebokehshape _boverride_lensflarethreshold _boverride_vignetteintensity _boverride_vignettecolor _boverride_grainintensity _boverride_grainjitter _boverride_ambientocclusionintensity _boverride_ambientocclusionstaticfraction _boverride_ambientocclusionradius _boverride_ambientocclusionfadedistance _boverride_ambientocclusionfaderadius _boverride_ambientocclusiondistance _boverride_ambientocclusionradiusinws _boverride_ambientocclusionpower _boverride_ambientocclusionbias _boverride_ambientocclusionquality _boverride_ambientocclusionmipblend _boverride_ambientocclusionmipscale _boverride_ambientocclusionmipthreshold _boverride_lpvintensity _boverride_lpvwarpintensity _boverride_lpvsize _boverride_lpvsecondaryocclusionintensity _boverride_lpvsecondarybounceintensity _boverride_lpvgeometryvolumebias _boverride_lpvvplinjectionbias _boverride_lpvemissiveinjectionintensity _boverride_lpvtransmissionintensity _boverride_indirectlightingcolor _boverride_indirectlightingintensity _boverride_colorgradingintensity _boverride_colorgradinglut _boverride_depthoffieldfocaldistance _boverride_depthoffieldfocalregion _boverride_depthoffieldneartransitionregion _boverride_depthoffieldfartransitionregion _boverride_depthoffieldscale _boverride_depthoffieldmaxbokehsize _boverride_depthoffieldnearblursize _boverride_depthoffieldfarblursize _boverride_depthoffieldmethod _boverride_depthoffieldbokehshape _boverride_depthoffieldocclusion _boverride_depthoffieldcolorthreshold _boverride_depthoffieldsizethreshold _boverride_depthoffieldskyfocusdistance _boverride_motionbluramount _boverride_motionblurmax _boverride_motionblurperobjectsize _boverride_screenpercentage _boverride_antialiasingmethod _boverride_screenspacereflectionintensity _boverride_screenspacereflectionquality _boverride_screenspacereflectionmaxroughness _boverride_screenspacereflectionroughnessscale _filmwhitepoint _filmshadowtint _filmshadowtintblend _filmshadowtintamount _filmsaturation _filmchannelmixerred _filmchannelmixergreen _filmchannelmixerblue _filmcontrast _filmtoeamount _filmhealamount _filmdynamicrange _scenecolortint _scenefringeintensity _scenefringesaturation _bloomintensity _bloomthreshold _bloom1size _bloom2size _bloom3size _bloom4size _bloom5size _bloom1tint _bloom2tint _bloom3tint _bloom4tint _bloom5tint _bloomdirtmaskintensity _bloomdirtmasktint _bloomdirtmask _lpvintensity _lpvwarpintensity _lpvvplinjectionbias _lpvsize _lpvsecondaryocclusionintensity _lpvsecondarybounceintensity _lpvgeometryvolumebias _lpvemissiveinjectionintensity _lpvtransmissionintensity _ambientcubemaptint _ambientcubemapintensity _ambientcubemap _autoexposurelowpercent _autoexposurehighpercent _autoexposureminbrightness _autoexposuremaxbrightness _autoexposurespeedup _autoexposurespeeddown _autoexposurebias _histogramlogmin _histogramlogmax _lensflareintensity _lensflaretint _lensflarebokehsize _lensflarethreshold _lensflarebokehshape _lensflaretints _vignetteintensity _vignettecolor _grainjitter _grainintensity _ambientocclusionintensity _ambientocclusionstaticfraction _ambientocclusionradius _ambientocclusionradiusinws _ambientocclusionfadedistance _ambientocclusionfaderadius _ambientocclusiondistance _ambientocclusionpower _ambientocclusionbias _ambientocclusionquality _ambientocclusionmipblend _ambientocclusionmipscale _ambientocclusionmipthreshold _indirectlightingcolor _indirectlightingintensity _colorgradingintensity _colorgradinglut _depthoffieldmethod _depthoffieldfocaldistance _depthoffieldfocalregion _depthoffieldneartransitionregion _depthoffieldfartransitionregion _depthoffieldscale _depthoffieldmaxbokehsize _depthoffieldnearblursize _depthoffieldfarblursize _depthoffieldbokehshape _depthoffieldocclusion _depthoffieldcolorthreshold _depthoffieldsizethreshold _depthoffieldskyfocusdistance _motionbluramount _motionblurmax _motionblurperobjectsize _screenpercentage _antialiasingmethod _screenspacereflectionintensity _screenspacereflectionquality _screenspacereflectionmaxroughness _blendables) (Utilities|Struct|BreakPostProcessSettings _postprocesssettings))
  (:Released
    (Utilities|Struct|SetmembersinPostProcessSettings _postprocesssettings _boverride_filmwhitepoint _boverride_filmsaturation _boverride_filmchannelmixerred _boverride_filmchannelmixergreen _boverride_filmchannelmixerblue _boverride_filmcontrast _boverride_filmdynamicrange _boverride_filmhealamount _boverride_filmtoeamount _boverride_filmshadowtint _boverride_filmshadowtintblend _boverride_filmshadowtintamount _boverride_scenecolortint _boverride_scenefringeintensity _boverride_scenefringesaturation _boverride_ambientcubemaptint _boverride_ambientcubemapintensity _boverride_bloomintensity _boverride_bloomthreshold _boverride_bloom1tint _boverride_bloom1size _boverride_bloom2size _boverride_bloom2tint _boverride_bloom3tint _boverride_bloom3size _boverride_bloom4tint _boverride_bloom4size _boverride_bloom5tint _boverride_bloom5size _boverride_bloomdirtmaskintensity _boverride_bloomdirtmasktint _boverride_bloomdirtmask _boverride_autoexposurelowpercent _boverride_autoexposurehighpercent _boverride_autoexposureminbrightness _boverride_autoexposuremaxbrightness _boverride_autoexposurespeedup _boverride_autoexposurespeeddown _boverride_autoexposurebias _boverride_histogramlogmin _boverride_histogramlogmax _boverride_lensflareintensity _boverride_lensflaretint _boverride_lensflaretints _boverride_lensflarebokehsize _boverride_lensflarebokehshape _boverride_lensflarethreshold _boverride_vignetteintensity _boverride_vignettecolor _boverride_grainintensity _boverride_grainjitter _boverride_ambientocclusionintensity _boverride_ambientocclusionstaticfraction _boverride_ambientocclusionradius _boverride_ambientocclusionfadedistance _boverride_ambientocclusionfaderadius _boverride_ambientocclusiondistance _boverride_ambientocclusionradiusinws _boverride_ambientocclusionpower _boverride_ambientocclusionbias _boverride_ambientocclusionquality _boverride_ambientocclusionmipblend _boverride_ambientocclusionmipscale _boverride_ambientocclusionmipthreshold _boverride_lpvintensity _boverride_lpvwarpintensity _boverride_lpvsize _boverride_lpvsecondaryocclusionintensity _boverride_lpvsecondarybounceintensity _boverride_lpvgeometryvolumebias _boverride_lpvvplinjectionbias _boverride_lpvemissiveinjectionintensity _boverride_lpvtransmissionintensity _boverride_indirectlightingcolor _boverride_indirectlightingintensity _boverride_colorgradingintensity true _boverride_depthoffieldfocaldistance _boverride_depthoffieldfocalregion _boverride_depthoffieldneartransitionregion _boverride_depthoffieldfartransitionregion _boverride_depthoffieldscale _boverride_depthoffieldmaxbokehsize _boverride_depthoffieldnearblursize _boverride_depthoffieldfarblursize _boverride_depthoffieldmethod _boverride_depthoffieldbokehshape _boverride_depthoffieldocclusion _boverride_depthoffieldcolorthreshold _boverride_depthoffieldsizethreshold _boverride_depthoffieldskyfocusdistance _boverride_motionbluramount _boverride_motionblurmax _boverride_motionblurperobjectsize _boverride_screenpercentage _boverride_antialiasingmethod _boverride_screenspacereflectionintensity _boverride_screenspacereflectionquality _boverride_screenspacereflectionmaxroughness _boverride_screenspacereflectionroughnessscale _filmwhitepoint _filmshadowtint _filmshadowtintblend _filmshadowtintamount _filmsaturation _filmchannelmixerred _filmchannelmixergreen _filmchannelmixerblue _filmcontrast _filmtoeamount _filmhealamount _filmdynamicrange _scenecolortint _scenefringeintensity _scenefringesaturation _bloomintensity _bloomthreshold _bloom1size _bloom2size _bloom3size _bloom4size _bloom5size _bloom1tint _bloom2tint _bloom3tint _bloom4tint _bloom5tint _bloomdirtmaskintensity _bloomdirtmasktint _bloomdirtmask _lpvintensity _lpvwarpintensity _lpvvplinjectionbias _lpvsize _lpvsecondaryocclusionintensity _lpvsecondarybounceintensity _lpvgeometryvolumebias _lpvemissiveinjectionintensity _lpvtransmissionintensity _ambientcubemaptint _ambientcubemapintensity _ambientcubemap _autoexposurelowpercent _autoexposurehighpercent _autoexposureminbrightness _autoexposuremaxbrightness _autoexposurespeedup _autoexposurespeeddown _autoexposurebias _histogramlogmin _histogramlogmax _lensflareintensity _lensflaretint _lensflarebokehsize _lensflarethreshold _lensflarebokehshape _lensflaretints _vignetteintensity _vignettecolor _grainjitter _grainintensity _ambientocclusionintensity _ambientocclusionstaticfraction _ambientocclusionradius _ambientocclusionradiusinws _ambientocclusionfadedistance _ambientocclusionfaderadius _ambientocclusiondistance _ambientocclusionpower _ambientocclusionbias _ambientocclusionquality _ambientocclusionmipblend _ambientocclusionmipscale _ambientocclusionmipthreshold _indirectlightingcolor _indirectlightingintensity _colorgradingintensity "/Game/Blueprints/blackandwhite.blackandwhite" _depthoffieldmethod _depthoffieldfocaldistance _depthoffieldfocalregion _depthoffieldneartransitionregion _depthoffieldfartransitionregion _depthoffieldscale _depthoffieldmaxbokehsize _depthoffieldnearblursize _depthoffieldfarblursize _depthoffieldbokehshape _depthoffieldocclusion _depthoffieldcolorthreshold _depthoffieldsizethreshold _depthoffieldskyfocusdistance _motionbluramount _motionblurmax _motionblurperobjectsize _screenpercentage _antialiasingmethod _screenspacereflectionintensity _screenspacereflectionquality _screenspacereflectionmaxroughness _blendables)))

(event Input|KeyboardEvents|F
  (:Pressed
    (Development|PrintString "Camera 2")
    (Components|Activation|SetActive (Variables|Default|GetSideViewCameraComponent) false true)))

(event EventActorEndOverlap
  (params (OtherActor :type Actor%20Object%20Reference))
  (if (Utilities|ClassIsChildOf (Utilities|GetClass OtherActor) "/Game/Blueprints/trap.Trap_C")
    (Variables|Default|SetinTrap false))
  (Variables|Default|Setcollision_count (- (Variables|Default|Getcollision_count) 1.0)))

(event EventActorBeginOverlap
  (params (OtherActor :type Actor%20Object%20Reference))
  (bind _returnvalue (Utilities|GetClass OtherActor))
  (Variables|Default|Setcollision_count (+ (Variables|Default|Getcollision_count) 1.0))
  (if (Utilities|ClassIsChildOf (Utilities|GetClass OtherActor) "/Game/Blueprints/trap.Trap_C")
    (Variables|Default|SetinTrap true))
  (if (<= (Variables|Default|Getcollision_count) 1.0)
    (Variables|Default|Setphase_start_location (Transformation|GetActorLocation)))
  ;[1 1 1] Check if collision is with trap, and check if the trap is phasible
  (if (not (Utilities|ClassIsChildOf _returnvalue "/Game/Blueprints/phasible.phasible_C"))
    (if (Utilities|ClassIsChildOf _returnvalue "/Game/Blueprints/trap.Trap_C")
      (if (not (and (Utilities|ClassIsChildOf _returnvalue "/Game/Blueprints/phasibile_trap.phasibile_trap_C") (Variables|Default|Getphase)))
        (Development|PrintString "1 Damage")
        (if (not (Variables|Default|Getdead))
          (Utilities|TakeDamage))))))

(fn ConstructionScript)