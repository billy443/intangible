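; CheckpointVolume is a checkpoint Blueprint meant to save player progress, but its ActorBeginOverlap event is unconnected, so none of its logic runs.
; The disconnected graph checks for Main_Character and copies CheckpointNumber onto the player character.
; It then creates a fresh GameSave with that number and the character's current level, and writes it to the save's own slot and user index.
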(event EventActorBeginOverlap
  (params (OtherActor :type Actor%20Object%20Reference)))

(fn ConstructionScript)