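; Solid 200x200 building Blueprint with a box and a static mesh, whose construction script is currently empty.
; An unconnected graph would create a dynamic instance of ScaledMaterial on the mesh.
; It would derive YThickness and XThickness from the box's Z and Y world scale, clamping border width between BorderMinPixels and BorderMinRatio so borders stay consistent on scaled buildings.
; None of this logic runs.
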(fn ConstructionScript)