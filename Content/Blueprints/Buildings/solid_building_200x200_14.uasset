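; Solid 200x200 building Blueprint with a static mesh and a box, whose construction script is empty.
; Disconnected, never-run logic would create a dynamic instance of ScaledMaterial on the mesh to keep border thickness bounded as the building scales.
; It derives YThickness and XThickness from the box's Z and Y world scale, overriding them only when a tenth of that size falls outside the BorderMinPixels to BorderMinRatio range.
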(fn ConstructionScript)