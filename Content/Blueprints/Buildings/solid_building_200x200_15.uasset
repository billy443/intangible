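; Solid building Blueprint, named as a 200x200 variant, whose construction script is currently empty.
; Disconnected, never-run logic would create a dynamic ScaledMaterial on StaticMesh1 to adjust border thickness to Box1's world scale.
; It would derive YThickness from Z scale and XThickness from Y scale, clamping border size between BorderMinPixels and BorderMinRatio, which acts as an upper limit.
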(fn ConstructionScript)