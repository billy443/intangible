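; Solid 200x200 building piece with a static mesh and box, whose Construction Script is empty.
; Disconnected, never-run logic would create a dynamic instance of ScaledMaterial to keep border widths consistent as the box scales.
; It derives YThickness from Z scale and XThickness from Y scale, overriding them when a tenth of the size falls below BorderMinPixels or exceeds BorderMinRatio, which acts as a maximum width.
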(fn ConstructionScript)