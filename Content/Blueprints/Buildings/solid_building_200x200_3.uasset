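; Solid 200x200 building Blueprint with a static mesh and box, whose construction script is empty.
; Unwired logic, which never runs, would create a dynamic instance of ScaledMaterial to keep borders consistent under scaling.
; It derives XThickness and YThickness from the box's Y and Z world scale, overriding them only when a tenth of the size falls outside the BorderMinPixels to BorderMinRatio range.
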(fn ConstructionScript)