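; A 200x200 solid building Blueprint with a box and a static mesh, whose construction script currently does nothing.
; Unconnected nodes would create a dynamic material from ScaledMaterial to keep border thickness in bounds as the box scales.
; They compare a tenth of the box's Y and Z size against BorderMinPixels and BorderMinRatio, then set XThickness and YThickness accordingly.
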(fn ConstructionScript)