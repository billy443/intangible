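; Solid 200x200 building Blueprint with a box and static mesh, whose construction script currently does nothing.
; Disconnected nodes would create a dynamic instance of ScaledMaterial on the mesh and set XThickness and YThickness from the box's Y and Z world scale.
; That unused logic clamps border thickness between BorderMinPixels and BorderMinRatio, the latter acting as a maximum despite its name, so borders would stay consistent as the building scales.
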(fn ConstructionScript)