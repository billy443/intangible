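; Solid 200x200 building piece whose construction script is empty, so it does nothing when constructed.
; Disconnected, never-run nodes would create a dynamic material on StaticMesh1 and set its border thickness from Box1's world scale.
; They would fit XThickness to Y scale and YThickness to Z scale, clamping the 10% border between BorderMinPixels and BorderMinRatio to keep it consistent as the box scales.
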(fn ConstructionScript)