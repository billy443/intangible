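; A solid building Blueprint whose construction script adapts the material border on its static mesh to the building's scale.
; It creates a dynamic instance of ScaledMaterial, then derives XThickness and YThickness from Box1's world Y and Z scale.
; When a tenth of either dimension falls outside the BorderMinPixels–BorderMinRatio range, thickness becomes that bound divided by the dimension; otherwise the material default stays.
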(fn ConstructionScript
  (bind _box1 (Variables|Default|GetBox1))
  (bind _box1_2 (Variables|Default|GetBox1))
  (bind _returnvalue (Transformation|GetWorldScale _box1))
  (bind _returnvalue_2 (Transformation|GetWorldScale _box1_2))
  (bind _y (Math|Vector|BreakVector _returnvalue))
  (bind _z (Math|Vector|BreakVector _returnvalue_2))
  (bind _returnvalue_3 (Rendering|Material|CreateDynamicMaterialInstance (Variables|Default|GetStaticMesh1) 0 (Variables|Default|Getscaled_material) :!class /Script/Engine.PrimitiveComponent))
  (Utilities|FlowControl|Sequence
    (:then_0
      (if (>= (* (* _z 2e+02) 0.1) (Variables|Default|Getborder_min_pixels))
        (if (> (* (* _z 2e+02) 0.1) (Variables|Default|Getborder_min_ratio))
          (Rendering|Material|SetScalarParameterValue _returnvalue_3 "YThickness" (/ (Variables|Default|Getborder_min_ratio) (* _z 2e+02)) :!class /Script/Engine.MaterialInstanceDynamic))
        (else
          (Rendering|Material|SetScalarParameterValue _returnvalue_3 "YThickness" (/ (Variables|Default|Getborder_min_pixels) (* _z 2e+02)) :!class /Script/Engine.MaterialInstanceDynamic))))
    (:then_1
      (if (>= (* (* _y 2e+02) 0.1) (Variables|Default|Getborder_min_pixels))
        (if (> (* (* _y 2e+02) 0.1) (Variables|Default|Getborder_min_ratio))
          (Rendering|Material|SetScalarParameterValue _returnvalue_3 "XThickness" (/ (Variables|Default|Getborder_min_ratio) (* _y 2e+02)) :!class /Script/Engine.MaterialInstanceDynamic))
        (else
          (Rendering|Material|SetScalarParameterValue _returnvalue_3 "XThickness" (/ (Variables|Default|Getborder_min_pixels) (* _y 2e+02)) :!class /Script/Engine.MaterialInstanceDynamic))))))