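; Enemy bot character that carries a socket-attached M16 and responds to enemy-found, enemy-lost and death events.
; On detection, unless the player's death flag is set, it plays firing animation and sound and spawns a trailed projectile, with a Firing flag and delay limiting fire rate.
; Losing the target restores the animation blueprint, and death plays an animation.
; Tick updates walk speed and a yaw-based facing flag, read only by disconnected vision-cone debug code.
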(event Custom|EnemyFound_Event
  (bind _returnvalue (Pawn|GetControlRotation :!class /Script/Engine.Pawn))
  (bind _mesh (Variables|Character|GetMesh))
  (if (not (Variables|Default|Getfiring))
    (Variables|Default|Setfiring true)
    (bind _death (Class|GetPlayerDeath|GetPlayerDeath(Message) (Game|GetPlayerCharacter 0)))
    (if (not _death)
      (Components|Animation|PlayAnimation _mesh "/Game/Animations/SWATAnimations/firing_rifle_1.firing_rifle_1" false)
      (Audio|PlaySoundatLocation "/Game/Particles/AssaultRifle_Shot01_Stereo.AssaultRifle_Shot01_Stereo" (Transformation|GetWorldLocation _mesh) 0.5)
      ;[1 1 1] Enemy Shooting (www.gog.gl/998Rox)
      (bind _returnvalue_2 (Game|SpawnActorfromClass "/Game/Blueprints/BotAI/Projectile.Projectile_C" (Math|Transform|MakeTransform (+ (Transformation|GetWorldLocation (Variables|Default|Getbullet_spawn_box)) (* (Math|Vector|GetForwardVector _returnvalue) (Variables|Default|Getbullet_speed)) "") _returnvalue "1.000000,1.000000,1") true 0))
      (Effects|SpawnEmitterAttached "/Game/Particles/P_Bullet_Trail.P_Bullet_Trail" (Variables|/Game/Blueprints/BotAI/Projectile.Projectile_C|GetSphere1 _returnvalue_2) "None")
      (Actor|SetLifeSpan _returnvalue_2 (Variables|Default|Getbullet_life_span))
      (Utilities|FlowControl|Delay (Variables|Default|Getfire_rate))
      (Variables|Default|Setfiring false))))

(event Custom|EnemyLost_Event
  (Components|Animation|SetAnimationMode (Variables|Character|GetMesh) "AnimationBlueprint"))

(event Custom|BotDeath_Event
  (Components|Animation|PlayAnimation (Variables|Character|GetMesh) "/Game/Animations/SWATAnimations/death_3.death_3" false))

(event EventBeginPlay)

(event EventTick
  (params (DeltaSeconds :type Float%20%28single-precision%29))
  (bind _mesh (Variables|Character|GetMesh))
  (bind _returnvalue (Transformation|GetWorldRotation _mesh))
  (bind _yaw (Class|KismetMathLibrary|BreakRot _returnvalue))
  (bind _returnvalue_2 (Math|Float|Round _yaw))
  (Variables|/Script/Engine.CharacterMovementComponent|SetMaxWalkSpeed (Variables|Character|GetCharacterMovement) (* (Variables|Default|GetspeedVariable) (Variables|Default|GetspeedRate)))
  (if (and (<= _returnvalue_2 0) (> _returnvalue_2 -90))
    (Variables|Default|Sethorizontal_rotation false)
    (else
      (Variables|Default|Sethorizontal_rotation true))))

(fn ConstructionScript
  (Class|SceneComponent|Attachto (Variables|Default|Getm16) (Variables|Character|GetMesh) "Gun" "KeepRelativeOffset"))

(fn GetPlayerDeath
  (return (Variables|Default|Getdeath)))