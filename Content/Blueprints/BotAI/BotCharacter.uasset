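; BotCharacter is an AI bot character that carries a sword and slashes when it finds an enemy.
; Enemy-found and enemy-lost events switch the mesh between a slash animation and its AnimBP, while Tick sets walk speed from two variables.
; TakeDamage decrements HP and plays a death animation at zero.
; Trap-hit logic is disconnected, and IsAttacking always returns false, ignoring the flag set by Attack input.
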(event Custom|EnemyFound_Event
  (Components|Animation|PlayAnimation (Variables|Character|GetMesh) "/Game/Character/Mixamo_Character_with_Sword/Animations/great_sword_slash_1.great_sword_slash_1" false))

(event Custom|EnemyLost_Event
  (Components|Animation|SetAnimationMode (Variables|Character|GetMesh) "AnimationBlueprint"))

(event EventActorEndOverlap
  (params (OtherActor :type Actor%20Object%20Reference))
  ;[1 1 1] If the collided object was a trap then reset the boolean flag
  (if (Utilities|ClassIsChildOf (Utilities|GetClass OtherActor) "/Game/Blueprints/Parents/Trap.Trap_C")
    _))

(event EventActorBeginOverlap
  (params (OtherActor :type Actor%20Object%20Reference)))

(event Input|ActionEvents|InputActionAttack
  ;[1 1 1] Set attacking based on attack button pushed
  (:Pressed
    (Variables|Default|Setattacking true))
  (:Released
    (Variables|Default|Setattacking false)))

(event EventTick
  (params (DeltaSeconds :type Float%20%28single-precision%29))
  (Variables|/Script/Engine.CharacterMovementComponent|SetMaxWalkSpeed (Variables|Character|GetCharacterMovement) (* (Variables|Default|GetspeedVariable) (Variables|Default|GetspeedRate))))

(fn ConstructionScript
  (Class|SceneComponent|Attachto (Variables|Default|GetSword) (Variables|Character|GetMesh) "SwordGrip" "KeepRelativeOffset"))

(fn NewFunction0)

(fn GetPlayerDeath
  ;[1 1 1] Get player death, used for player animation blueprint
  (return (Variables|Default|Getdead)))

(fn IsAttacking
  ;[1 1 1] Get if player is attacking, used for character animation blueprint
  (return false))