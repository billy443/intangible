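; AI controller for enemy bots that starts their behavior tree when play begins.
; On BeginPlay it loads the BotData blackboard and casts the controlled pawn to EnemyAI, stopping if that fails.
; It copies the pawn's WaypointIndex into the EnemyNumber key, then runs BotAITree.
; A debug print of the index is left disconnected.
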(event EventBeginPlay
  ;[1 1 1] Initialize Bot AI
  (Class|AIController|UseBlackboard "/Game/Blueprints/BotAI/BotData.BotData")
  (bind _asenemyai_c (Utilities|Casting|CastToEnemyAI (Pawn|GetControlledPawn)))
  (Class|BlackboardComponent|SetValueasInt (AI|GetBlackboard self) (Variables|Default|GetEnemyNumber) (Variables|/Game/Blueprints/BotAI/EnemyAI.EnemyAI_C|Getwaypoint_index _asenemyai_c))
  (AI|RunBehaviorTree "/Game/Blueprints/BotAI/BotAITree.BotAITree"))

(fn ConstructionScript)