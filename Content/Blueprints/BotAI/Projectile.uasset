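; Projectile actor that deals heavy damage to the player character or enemy AI it overlaps, then destroys itself.
; Overlapping either class opens a Tick-fed gate that applies the damage on a following tick, and ending the overlap closes it.
; Overlaps with any other actor destroy it immediately, and the Hit event also destroys it after a similar class check.
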(event EventHit
  (params (MyComp :type Primitive%20Component%20Object%20Reference) (Other :type Actor%20Object%20Reference) (OtherComp :type Primitive%20Component%20Object%20Reference) (bSelfMoved :type Boolean) (HitLocation :type Vector :default "0, 0, 0") (HitNormal :type Vector :default "0, 0, 0") (NormalImpulse :type Vector :default "0, 0, 0") (Hit :type Hit%20Result%20Structure%20%28by%20ref%29))
  (if (not (or (== (Utilities|GetClass (stale EventActorBeginOverlap OtherActor)) "/Game/Blueprints/Main_Character.Main_Character_C") (== (Utilities|GetClass (stale EventActorBeginOverlap OtherActor)) "/Game/Blueprints/BotAI/EnemyAI.EnemyAI_C")))
    (Actor|DestroyActor)))

(event EventActorBeginOverlap
  (params (OtherActor :type Actor%20Object%20Reference))
  (bind _returnvalue (Utilities|GetClass OtherActor))
  (if (or (== _returnvalue "/Game/Blueprints/Main_Character.Main_Character_C") (== _returnvalue "/Game/Blueprints/BotAI/EnemyAI.EnemyAI_C"))
    (Utilities|FlowControl|Gate true) ; enters at Open
    (else
      ;[1 1 1] Destroys projectiles after hitting target
      (Actor|DestroyActor self))))

(event EventTick
  (params (DeltaSeconds :type Float%20%28single-precision%29))
  (Utilities|FlowControl|Gate true
    (:Exit
      (Game|Damage|ApplyDamage (stale EventActorBeginOverlap OtherActor) 1e+02 0 0 "/Script/Engine.DamageType")
      ;[1 1 1] Destroys projectiles after hitting target
      (Actor|DestroyActor self))))

(event EventActorEndOverlap
  (params (OtherActor :type Actor%20Object%20Reference))
  (Utilities|FlowControl|Gate true) ; enters at Close
)

(fn ConstructionScript)