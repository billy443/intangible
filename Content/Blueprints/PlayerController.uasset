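; Player controller that toggles a pause menu on the Pause input action.
; A FlipFlop alternates between opening and closing, with opening requiring the pawn to be a Main_Character.
; Opening spawns a Menu actor at the character's location, gives it input, shows the cursor with click events and pauses the game.
; Closing reverses those settings, unpauses and destroys the menu.
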(event Input|ActionEvents|InputActionPause
  (bind _returnvalue (Game|GetPlayerController 0))
  (:Pressed
    (Utilities|FlowControl|FlipFlop
      (:A
        (bind _asmain_character_c (Utilities|Casting|CastToMain_Character (Game|Player|GetPlayerPawn 0)))
        (bind _returnvalue_2 (Game|SpawnActorfromClass "/Game/Blueprints/Menu.Menu_C" (Math|Conversions|ToTransform(Vector) (Transformation|GetActorLocation _asmain_character_c)) true 0))
        (Variables|/Script/Engine.PlayerController|SetbEnableClickEvents _returnvalue true)
        (Variables|/Script/Engine.PlayerController|SetbShowMouseCursor _returnvalue true)
        (Input|EnableInput _returnvalue_2 _returnvalue)
        (Game|SetGamePaused true))
      (:B
        (Variables|/Script/Engine.PlayerController|SetbEnableClickEvents _returnvalue false)
        (Variables|/Script/Engine.PlayerController|SetbShowMouseCursor _returnvalue false)
        (Input|DisableInput _returnvalue_2 self)
        (Game|SetGamePaused false)
        (Actor|DestroyActor _returnvalue_2)))))

(fn ConstructionScript)