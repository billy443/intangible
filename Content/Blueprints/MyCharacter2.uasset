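; MyCharacter2 is a side-scroller player character with a meter-limited phase ability for passing through phasable objects and traps.
; Phasing changes time dilation, movement stats, jump gravity, capsule object type and the visible mesh and sword, while Tick drains or refills the meter.
; Overlap tracking kills on traps or, when phasing ends inside an object, moves the player out.
; A snap-back button teleports to a saved location; post-process effects are unfinished.
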(event EventOnLanded
  (params (Hit :type Hit%20Result%20Structure%20%28by%20ref%29))
  ;[1 1 1] Set the gravity based on the phase state when the jump was initiated, reset on landing
  (if (not (Variables|Default|Getis_phasing))
    (Variables|/Script/Engine.CharacterMovementComponent|SetGravityScale (Variables|Character|GetCharacterMovement) (Variables|Default|Getnormal_gravity))))

(event EventOnJumped
  (bind _charactermovement (Variables|Character|GetCharacterMovement))
  ;[1 1 1] Set the gravity based on the phase state when the jump was initiated, reset on landing
  (if (Variables|Default|Getis_phasing)
    (Variables|/Script/Engine.CharacterMovementComponent|SetGravityScale _charactermovement (Variables|Default|Getphase_gravity))
    (else
      (Variables|/Script/Engine.CharacterMovementComponent|SetGravityScale _charactermovement (Variables|Default|Getnormal_gravity)))))

(event Input|ActionEvents|InputActionphase
  ;[1 1 1] TODO: Will change the post processing effect (blank and white or tinted, etc.)  The camera provided with the 2D sidescroller template does not allow altering post processing effects from blueprints.
)

(event EventActorEndOverlap
  (params (OtherActor :type Actor%20Object%20Reference))
  ;[1 1 1] If the collided object was a trap then reset the boolean flag
  (if (Utilities|ClassIsChildOf (Utilities|GetClass OtherActor) "/Game/Blueprints/Parents/Trap.Trap_C")
    (Variables|Default|SetinTrap false))
  ;[1 1 1] Pop collision count
  (Variables|Default|Setcollision_count (- (Variables|Default|Getcollision_count) 0.5)))

(event EventActorBeginOverlap
  (params (OtherActor :type Actor%20Object%20Reference))
  (bind _returnvalue (Utilities|GetClass OtherActor))
  ;[1 1 1] Increment number of object colliding
  (Variables|Default|Setcollision_count (+ (Variables|Default|Getcollision_count) 0.5))
  ;[1 1 1] If object is a trap, flag as colliding with a trap
  (if (Utilities|ClassIsChildOf (Utilities|GetClass OtherActor) "/Game/Blueprints/Parents/Trap.Trap_C")
    (Variables|Default|SetinTrap true))
  ;[1 1 1] If this is the first collision save where the player entered the object
  (if (<= (Variables|Default|Getcollision_count) 0.5)
    (Variables|Default|Setphase_start_location (Transformation|GetActorLocation)))
  ;[1 1 1] Check if collision is with trap, and check if the trap is phasible
  (if (not (Utilities|ClassIsChildOf _returnvalue "/Game/Blueprints/Parents/phasable.phasable_C"))
    (if (Utilities|ClassIsChildOf _returnvalue "/Game/Blueprints/Parents/Trap.Trap_C")
      (if (not (and (Utilities|ClassIsChildOf _returnvalue "/Game/Blueprints/Parents/phasabile_trap.phasabile_trap_C") (Variables|Default|Getis_phasing)))
        ;[1 1 1] If the player isn't already dead apply damage (no death throws)
        (if (not (Variables|Default|Getdead))
          (Utilities|TakeDamage))))))

(event Custom|PhaseButtonPressed
  (bind _charactermovement (Variables|Character|GetCharacterMovement))
  (bind _phase_time_dilation (Variables|Default|Getphase_time_dilation))
  ;[1 1 1] Check if the player can phase
  (if (Variables|Default|Getcan_phase)
    ;[1 1 1] Set boolean flag for phase status
    (Variables|Default|Setis_phasing true)
    (Utilities|SpawnSnapBack
      (:FlowOut
        ;[1 1 1] Enable/Disable Time Dilation
        (Utilities|Time|SetGlobalTimeDilation _phase_time_dilation)
        (Variables|Default|SetCustomTimeDilation (/ 1.0 _phase_time_dilation))
        ;[1 1 1] Enable/Disable Phase Movement Changes
        (Variables|/Script/Engine.CharacterMovementComponent|SetMaxWalkSpeed _charactermovement (Variables|Default|Getphase_walk_speed))
        (Variables|/Script/Engine.CharacterMovementComponent|SetMaxAcceleration _charactermovement (Variables|Default|Getphase_acceleration))
        (Variables|/Script/Engine.CharacterMovementComponent|SetJumpZVelocity _charactermovement (Variables|Default|Getphase_jump_velocity))
        ;[1 1 1] Set graphic changes to player from based on phase state, toggle active mesh
        (Utilities|EnablePhaseGraphics
          (:FlowOut
            ;[1 1 1] Set player collision based on phase state
            (Collision|SetCollisionObjectType (Variables|/Script/Engine.Character|GetCapsuleComponent (Game|GetPlayerCharacter 0)) "ECC_Vehicle")))))))

(event Custom|PhaseButtonReleased
  (bind _charactermovement (Variables|Character|GetCharacterMovement))
  (bind _normal_time_dilation (Variables|Default|Getnormal_time_dilation))
  ;[1 1 1] Check if player is phasing
  (if (Variables|Default|Getis_phasing)
    ;[1 1 1] Set boolean flag for phase status
    (Variables|Default|Setis_phasing false)
    ;[1 1 1] Enable/Disable Time Dilation
    (Utilities|Time|SetGlobalTimeDilation _normal_time_dilation)
    (Variables|Default|SetCustomTimeDilation _normal_time_dilation)
    ;[1 1 1] Enable/Disable Phase Movement Changes
    (Variables|/Script/Engine.CharacterMovementComponent|SetMaxWalkSpeed _charactermovement (Variables|Default|Getnormal_walk_speed))
    (Variables|/Script/Engine.CharacterMovementComponent|SetMaxAcceleration _charactermovement (Variables|Default|Getnormal_acceleration))
    (Variables|/Script/Engine.CharacterMovementComponent|SetJumpZVelocity _charactermovement (Variables|Default|Getnormal_jump_velocity))
    ;[1 1 1] Set graphic changes to player from based on phase state, toggle active mesh
    (Utilities|DisablePhaseGraphics
      (:FlowOut
        ;[1 1 1] Set player collision based on phase state
        (Collision|SetCollisionObjectType (Variables|/Script/Engine.Character|GetCapsuleComponent (Game|GetPlayerCharacter 0)) "ECC_Pawn")
        ;[1 1 1] Check if the player is inside an object, if so and the object is a trap apply damage (death), otherwise move them out.
        (if (and (not (Variables|Default|GetinTrap)) (> (Variables|Default|Getcollision_count) 0.0))
          (Utilities|MovePlayerOverTime
            (:FlowOut
              (CallFunction|PhaseButtonReleased)))
          (elif (Variables|Default|GetinTrap)
            (Utilities|TakeDamage)))))))

(event Input|ActionEvents|InputActionphase
  (:Pressed
    ;[1 1 1] Set if the phase button is being held
    (Variables|Default|Setphase_button_held true)
    ;[1 1 1] Check if the player can phase
    (if (Variables|Default|Getcan_phase)
      (CallFunction|PhaseButtonPressed)))
  (:Released
    (Variables|Default|Setphase_button_held false)
    ;[1 1 1] Check if the player has enough phase meter and set if they can phase
    (if (< (Variables|Default|Getphase_meter) (Variables|Default|Getphase_meter_min))
      (Variables|Default|Setcan_phase false))
    ;[1 1 1] Check if player is phasing
    (if (Variables|Default|Getis_phasing)
      (CallFunction|PhaseButtonReleased))))

(event Input|ActionEvents|InputActionScreenshot
  (:Pressed
    (Development|ExecuteConsoleCommand "shot")))

(event Input|ActionEvents|InputActionAttack
  ;[1 1 1] Set attacking based on attack button pushed
  (:Pressed
    (Variables|Default|Setattacking true))
  (:Released
    (Variables|Default|Setattacking false)))

(event EventTick
  (params (DeltaSeconds :type Float%20%28single-precision%29))
  (bind _phase_meter_empty (Variables|Default|Getphase_meter_empty))
  (bind _phase_meter_max (Variables|Default|Getphase_meter_max))
  ;[1 1 1] Set can phase if player can phase and couldn't on previous tick
  (if (and (> (Variables|Default|Getphase_meter) (Variables|Default|Getphase_meter_min)) (not (Variables|Default|Getcan_phase)))
    (Variables|Default|Setcan_phase true))
  ;[1 1 1] Check if the player is phasing to set charging or depletion of meter
  (if (Variables|Default|Getcan_phase)
    (if (Variables|Default|Getis_phasing)
      ;[1 1 1] Decrease meter by delta time since last tick
      (Variables|Default|Setphase_meter (- (Variables|Default|Getphase_meter) DeltaSeconds))
      ;[1 1 1] Check if phase meter is empty and kick them out of phase if it is
      (if (<= (Variables|Default|Getphase_meter) _phase_meter_empty)
        (Variables|Default|Setphase_meter _phase_meter_empty)
        (Variables|Default|Setcan_phase false)
        (CallFunction|PhaseButtonReleased))
      (else
        ;[1 1 1] Increase meter by delta time since last tick
        (Variables|Default|Setphase_meter (+ (Variables|Default|Getphase_meter) DeltaSeconds) :!label _label)
        ;[1 1 1] Keep meter at or below max meter
        (if (>= (Variables|Default|Getphase_meter) _phase_meter_max)
          (Variables|Default|Setphase_meter _phase_meter_max))
        ;[1 1 1] Check if the button is already being held after increment
        (if (and (Variables|Default|Getphase_button_held) (Variables|Default|Getcan_phase))
          (CallFunction|PhaseButtonPressed))))
    (else
      (goto _label))))

(event EventBeginPlay
  ;[1 1 1] When the level loads set phase meter to full
  (Variables|Default|Setphase_meter (Variables|Default|Getphase_meter_max)))

(event Input|ActionEvents|InputActionSnapBack
  (:Pressed
    ;[1 1 1] If there is at least one snap back location object saved get the first one spawned, set the player's location to that object then destory snap back location object
    (bind _outactors (Actor|GetAllActorsOfClass "/Game/Blueprints/SnapBackLocation.SnapBackLocation_C"))
    (if (not (< (Utilities|Array|Length _outactors) 1))
      (Transformation|SetActorLocation (Transformation|GetActorLocation (Utilities|Array|Get(acopy) _outactors)) false)
      (Actor|DestroyActor (Utilities|Array|Get(acopy) _outactors)))))

(fn ConstructionScript
  ;[1 1 1] Attach sword to player mesh, and phase sword to phase player mesh
  (Class|SceneComponent|Attachto (Variables|Default|GetSword) (Variables|Character|GetMesh) "SwordGrip" "KeepRelativeOffset")
  (Class|SceneComponent|Attachto (Variables|Default|GetPhaseSword) (Variables|Default|GetPhaseMesh) "SwordGrip" "KeepRelativeOffset"))

(fn MoveIncrement
  (bind _returnvalue (Transformation|GetActorLocation))
  (bind (_x _y _z) (Math|Vector|BreakVector _returnvalue))
  ;[1 1 1] Move character once based on Y and Z deltas determined
  (Transformation|SetActorLocation (Math|Vector|MakeVector _x (- _y (Variables|Default|Gety_delta)) (- _z (Variables|Default|Getz_delta))) false))

(fn NewFunction0)

(fn GetPhaseMeter
  ;[1 1 1] Interface to get the phase meter, used for the HUD to get phase meter settings
  (return (Variables|Default|Getphase_meter) (Variables|Default|Getphase_meter_max) (Variables|Default|Getphase_meter_min)))

(fn GetPhasing
  ;[1 1 1] Return phasing status
  (return (Variables|Default|Getis_phasing)))

(fn GetPlayerDeath
  ;[1 1 1] Get player death, used for player animation blueprint
  (return (Variables|Default|Getdead)))

(fn IsAttacking
  ;[1 1 1] Get if player is attacking, used for character animation blueprint
  (return (Variables|Default|Getattacking)))